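; Fan affector that spins its blade mesh and pushes objects that enter its push volume.
; A Timeline started on BeginPlay drives the blade pitch, scaled by a speed variable.
; Overlap begin stores the component and starts a looping timer that applies impulses along a reference component's forward vector and prints debug text.
; Overlap end clears the timer; only the latest component and timer handle are stored.
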(event OnComponentBeginOverlap(PushCollBox)
  (params (OverlappedComponent :type Primitive%20Component%20Object%20Reference) (OtherActor :type Actor%20Object%20Reference) (OtherComp :type Primitive%20Component%20Object%20Reference) (OtherBodyIndex :type Integer) (bFromSweep :type Boolean) (SweepResult :type Hit%20Result%20Structure%20%28by%20ref%29))
  ;[0.6729 1 0.6653] FanPush
  ;;[1 1 1] Begin Overlap
  (Variables|Default|SetOverlapped%20Component OverlappedComponent)
  (Variables|Default|SetOther%20Actor OtherActor)
  (Variables|Default|SetOther%20Comp_0 OtherComp)
  (bind _returnvalue (Utilities|Time|SetTimerbyEvent (delegate Custom|OnPushUpdate) (Variables|Default|GetPushUpdateTimeInc) true))
  (Variables|Default|SetTimerHandle _returnvalue))

(event OnComponentEndOverlap(PushCollBox)
  (params (OverlappedComponent :type Primitive%20Component%20Object%20Reference) (OtherActor :type Actor%20Object%20Reference) (OtherComp :type Primitive%20Component%20Object%20Reference) (OtherBodyIndex :type Integer))
  ;[0.6729 1 0.6653] FanPush
  ;;[1 1 1] End Overlap
  (Utilities|Time|ClearandInvalidateTimerbyHandle (Variables|Default|GetTimerHandle)))

(event Custom|OnPushUpdate
  (bind _pushmulti (Variables|Default|GetPushMulti))
  (bind _other_comp_0 (Variables|Default|GetOther%20Comp_0))
  (bind _vectorthing (Variables|Default|GetVectorthing))
  (bind _returnvalue (Math|Vector|GetForwardVector _vectorthing))
  (bind _returnvalue_2 (* _returnvalue _pushmulti))
  (bind (_x _y _z) (Math|Vector|BreakVector _returnvalue_2))
  ;[0.6729 1 0.6653] FanPush
  ;;[1 1 1] Begin Overlap
  ;;[0 0 0] Impulse
  (Physics|AddImpulse _other_comp_0 _returnvalue_2 "None" false)
  (Development|PrintText (Utilities|Text|FormatText "Impulse Vector: ({X},{Y},{Z}) Subject {S}" _x _y _z _other_comp_0)))

(event EventBeginPlay
  ;[1 1 1] Fan Rotation
  (bind _fanrotation (Timeline|Timeline Play)
    (:Update
      (Transformation|SetRelativeRotation (Variables|Default|GetFan01_Fan) (Math|Rotator|MakeRotator 0.0 (* _fanrotation (Variables|Default|GetFANSPEED)) 0.0) false false))))

(event EventTick
  (params (DeltaSeconds :type Float%20%28single-precision%29)))

(fn ConstructionScript)