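; Swinging hammer actor, in a developer test folder, that swings its HammerDiveHandle component back and forth like a pendulum.
; BeginPlay caches the handle's relative location as the base vector.
; Each Tick feeds a time value into a pulsating value that blends between the swing start and end angles.
; That angle drives both the handle's roll and its position, rotated about an X axis through an offset pivot on Z.
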(event EventBeginPlay
  ;[1 1 1] Calculate the location of the hammer
  (bind _output_get (Variables|Default|SetRelative%20Location (Variables|/Script/Engine.SceneComponent|GetRelativeLocation (Variables|Default|Gethammer_Dive_handle)))))

(event Collision|EventActorBeginOverlap
  (params (OtherActor :type Actor%20Object%20Reference)))

(event EventTick
  (params (DeltaSeconds :type Float%20%28single-precision%29))
  ;[1 1 1] Make a sin wave
  (bind _output_get (Variables|Default|SetDelta%20Seconds (+ DeltaSeconds (Variables|Default|GetDelta%20Seconds))))
  ;[1 1 1] Make angles
  (bind _result (Math|Float|NegateFloat (Math|Float|Lerp (Variables|Default|GetSwingStart) (Variables|Default|GetSwingEnd) (Class|KismetMathLibrary|MakePulsatingValue _output_get (Variables|Default|GetIn%20Pulses%20Per%20Second) (Variables|Default|GetIn%20Phase))))
    (:%20%20
      (Transformation|SetRelativeLocationAndRotation (Variables|Default|Gethammer_Dive_handle) (Utilities|RotateVectorAroundNon-worldAxis (Math|Vector|MakeVector 1e+01 0.0 0.0) (Math|Vector|MakeVector 0.0 0.0 6e+02) (stale EventBeginPlay _output_get) (Math|Float|Lerp (Variables|Default|GetSwingStart) (Variables|Default|GetSwingEnd) (Class|KismetMathLibrary|MakePulsatingValue _output_get (Variables|Default|GetIn%20Pulses%20Per%20Second) (Variables|Default|GetIn%20Phase)))) (Math|Rotator|MakeRotator _result 0.0 0.0) false false))))

(fn ConstructionScript)